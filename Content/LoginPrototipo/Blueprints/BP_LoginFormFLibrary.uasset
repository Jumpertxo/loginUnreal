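; Blueprint function library for the login form prototype, providing screen switching, login playback and theming of its UI.
; MasterRef casts player pawn 0 to BP_LoginFormPrototype to reach its master and intro widgets.
; SwitchWidget animates and changes the switcher index, while LogInEvent triggers login and returns its animation end time.
; PrimaryColor, PlayButton and Intro apply passed-in style settings to buttons, borders, loading bars, text and backgrounds.
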(fn SwitchWidget
  (params (Index :type Integer) (StartAtTime :type Float%20%28double-precision%29) (PlaybackSpeed :type Float%20%28double-precision%29) (PlayMode :type EUMGSequencePlayMode%20Enum :default "Forward"))
  ;[1 0 0.07113] Switch Widget
  (bind _asbp_login_form_prototype (Utilities|Casting|CastToBP_LoginFormPrototype (Game|Player|GetPlayerPawn 0)))
  (UserInterface|Animation|PlayAnimation (Variables|/Game/LoginPrototipo/Blueprints/BP_LoginFormPrototype.BP_LoginFormPrototype_C|GetWBP_Master _asbp_login_form_prototype) (Variables|/Game/LoginPrototipo/Widgets/WBP_Master.WBP_Master_C|GetWidgetSwitcher (Variables|/Game/LoginPrototipo/Blueprints/BP_LoginFormPrototype.BP_LoginFormPrototype_C|GetWBP_Master _asbp_login_form_prototype)) StartAtTime 1 PlayMode PlaybackSpeed false)
  (Class|WidgetSwitcher|SetActiveWidgetIndex (Variables|/Game/LoginPrototipo/Widgets/WBP_Master.WBP_Master_C|GetBPWidgetSwitcher (Variables|/Game/LoginPrototipo/Blueprints/BP_LoginFormPrototype.BP_LoginFormPrototype_C|GetWBP_Master _asbp_login_form_prototype)) Index))

(fn LoginEvent
  (bind _ref (Reference|MasterRef))
  (bind _wbp_master (Variables|/Game/LoginPrototipo/Blueprints/BP_LoginFormPrototype.BP_LoginFormPrototype_C|GetWBP_Master _ref))
  ;[1 0 0.07113] Login Event
  (Utilities|IsValid _ref
    (:Is%20Valid
      (Default|LoginEvent _wbp_master)
      (return (Class|WidgetAnimation|GetEndTime (Variables|/Game/LoginPrototipo/Widgets/WBP_Master.WBP_Master_C|GetLogIn _wbp_master))))))

(fn MasterRef
  ;[1 0 0.07113] Master Reference
  (bind _asbp_login_form_prototype (Utilities|Casting|CastToBP_LoginFormPrototype (Game|Player|GetPlayerPawn 0)))
  (return _asbp_login_form_prototype))

(fn PrimaryColor
  (params (Reference :type F%20Primary%20Color%20Structure))
  (bind (_normalprimary _hoveredprimary _pressedprimary _primaryborder _loading) (Utilities|Struct|BreakF_PrimaryColor Reference))
  (bind _ref (Reference|MasterRef))
  (bind _wbp_master (Variables|/Game/LoginPrototipo/Blueprints/BP_LoginFormPrototype.BP_LoginFormPrototype_C|GetWBP_Master _ref))
  (bind _wbp_signup (Variables|/Game/LoginPrototipo/Widgets/WBP_Master.WBP_Master_C|GetWBP_SignUp _wbp_master))
  (bind _wbp_signin (Variables|/Game/LoginPrototipo/Widgets/WBP_Master.WBP_Master_C|GetWBP_SignIn _wbp_master))
  (bind _wbp_forgotpassword (Variables|/Game/LoginPrototipo/Widgets/WBP_Master.WBP_Master_C|GetWBP_ForgotPassword _wbp_master))
  ;[1 0 0.07113] PrimaryColor
  (Utilities|IsValid _ref
    (:Is%20Valid
      (Utilities|FlowControl|Sequence
        (:then_0
          (for _array_element (Utilities|Array|MakeArray (Variables|/Game/LoginPrototipo/Widgets/WBP_SignIn.WBP_SignIn_C|GetSignInButton _wbp_signin) (Variables|/Game/LoginPrototipo/Widgets/WBP_SignIn.WBP_SignIn_C|GetCreateNewAccountButton _wbp_signin) (Variables|/Game/LoginPrototipo/Widgets/WBP_SignUp.WBP_SignUp_C|GetContinue _wbp_signup) (Variables|/Game/LoginPrototipo/Widgets/WBP_SignUp.WBP_SignUp_C|GetBack _wbp_signup) (Variables|/Game/LoginPrototipo/Widgets/WBP_ForgotPassword.WBP_ForgotPassword_C|GetSignIn _wbp_forgotpassword) (Variables|/Game/LoginPrototipo/Widgets/WBP_ForgotPassword.WBP_ForgotPassword_C|GetSendEmail _wbp_forgotpassword))
            (Class|Button|SetStyle _array_element (|Color (Variables|/Script/UMG.Button|GetWidgetStyle _array_element) _normalprimary _hoveredprimary _pressedprimary))))
        (:then_1
          (Appearance|SetColorandOpacity (Variables|/Game/LoginPrototipo/Widgets/WBP_Master.WBP_Master_C|GetB2 _wbp_master) _primaryborder :!class /Script/UMG.Image)
          (Class|ProgressBar|SetFillColorandOpacity (Variables|/Game/LoginPrototipo/Widgets/WBP_Master.WBP_Master_C|GetLoadingProgressBar _wbp_master) _loading))))))

(fn PlayButton
  (params (Reference :type F%20Play%20Structure))
  (bind (_normal _hovered _pressed _fontsize _textcolor _text) (Utilities|Struct|BreakF_Play Reference))
  (bind _ref (Reference|MasterRef))
  (bind _wbp_master (Variables|/Game/LoginPrototipo/Blueprints/BP_LoginFormPrototype.BP_LoginFormPrototype_C|GetWBP_Master _ref))
  (bind _playbutton (Variables|/Game/LoginPrototipo/Widgets/WBP_Master.WBP_Master_C|GetPlayButton _wbp_master))
  (bind _playtext (Variables|/Game/LoginPrototipo/Widgets/WBP_Master.WBP_Master_C|GetPlayText _wbp_master))
  (bind _font (Variables|/Script/UMG.TextBlock|GetFont _playtext))
  (bind (_fontobject _fontmaterial _outlinesettings _typefacefontname _letterspacing) (Utilities|Struct|BreakSlateFontInfo _font))
  ;[1 0 0.07113] Play Button
  (Utilities|IsValid _ref
    (:Is%20Valid
      (Class|Button|SetStyle _playbutton (|Color (Variables|/Script/UMG.Button|GetWidgetStyle _playbutton) _normal _hovered _pressed))
      (Class|TextBlock|SetFont _playtext (Utilities|Struct|MakeSlateFontInfo _fontobject _fontmaterial _outlinesettings _typefacefontname _fontsize _letterspacing 0.0))
      (Appearance|SetColorandOpacity _playtext (Utilities|Struct|MakeSlateColor _textcolor "UseColor_Specified") :!class /Script/UMG.TextBlock)
      (Rendering|Components|TextRender|SetText _playtext _text))))

(fn Intro
  (params (Intro :type F%20Intro%20Structure))
  (bind (_backgroundcolor _backgroundimage _introtext _introtextfontsize _introtextcolor _loadingcolor) (Utilities|Struct|BreakF_Intro Intro))
  (bind _ref (Reference|MasterRef))
  (bind _wbp_intro (Variables|/Game/LoginPrototipo/Blueprints/BP_LoginFormPrototype.BP_LoginFormPrototype_C|GetWBP_Intro _ref))
  (bind _introtext_2 (Variables|/Game/LoginPrototipo/Widgets/WBP_Intro.WBP_Intro_C|GetIntroText _wbp_intro))
  (bind _font (Variables|/Script/UMG.TextBlock|GetFont _introtext_2))
  (bind (_fontobject _fontmaterial _outlinesettings _typefacefontname _letterspacing) (Utilities|Struct|BreakSlateFontInfo _font))
  ;[1 0 0.07113] Intro
  (Class|TextBlock|SetFont _introtext_2 (Utilities|Struct|MakeSlateFontInfo _fontobject _fontmaterial _outlinesettings _typefacefontname _introtextfontsize _letterspacing))
  (Appearance|SetBrushfromTexture (Variables|/Game/LoginPrototipo/Widgets/WBP_Intro.WBP_Intro_C|GetBackgroundImage _wbp_intro) _backgroundimage)
  (Class|Border|SetBrushColor (Variables|/Game/LoginPrototipo/Widgets/WBP_Intro.WBP_Intro_C|GetIntroBorder _wbp_intro) _backgroundcolor)
  (Class|ProgressBar|SetFillColorandOpacity (Variables|/Game/LoginPrototipo/Widgets/WBP_Intro.WBP_Intro_C|GetIntroLoading _wbp_intro) _loadingcolor)
  (Rendering|Components|TextRender|SetText _introtext_2 _introtext)
  (Appearance|SetColorandOpacity _introtext_2 (Utilities|Struct|MakeSlateColor _introtextcolor "UseColor_Specified") :!class /Script/UMG.TextBlock))