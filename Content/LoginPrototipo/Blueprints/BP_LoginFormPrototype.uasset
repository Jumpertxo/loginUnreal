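; BP_LoginFormPrototype is the entry point that puts the prototype login form UI on screen at BeginPlay.
; If enabled in the Intro settings, it shows a configured WBP_Intro widget and waits briefly before continuing.
; It then creates WBP_Master from the hint and background structures, adds it to the viewport and shows the mouse cursor.
; Primary color and play button setup calls exist but are unconnected.
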(event EventBeginPlay
  ;[1 0 0.07113] Begin Play
  (if (Utilities|Struct|BreakF_Intro (Variables|Default|GetIntro))
    (bind _returnvalue (UserInterface|CreateWidget "/Game/LoginPrototipo/Widgets/WBP_Intro.WBP_Intro_C"))
    (bind _output_get (Variables|Default|SetWBP_Intro _returnvalue))
    (CallFunction|Intro (Variables|Default|GetIntro))
    (UserInterface|Viewport|AddtoViewport _output_get 0)
    (Utilities|FlowControl|Delay 2.25))
  (bind _returnvalue_2 (UserInterface|CreateWidget "/Game/LoginPrototipo/Widgets/WBP_Master.WBP_Master_C" 0 (Variables|Default|GetHintStructure) (Variables|Default|GetBackground)))
  (bind _output_get_2 (Variables|Default|SetWBP_Master _returnvalue_2))
  (UserInterface|Viewport|AddtoViewport _output_get_2 0)
  (Variables|/Script/Engine.PlayerController|SetbShowMouseCursor (Game|GetPlayerController 0) true))

(fn ConstructionScript)